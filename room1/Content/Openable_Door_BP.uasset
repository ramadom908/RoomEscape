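; Openable door actor that swings open and closed in response to open and close requests from its OpenDoor component.
; The DoorSwing timeline interpolates actor rotation from the rotation cached at BeginPlay to a target rotator, playing forward to open and reversing to close.
; A sound event track on the timeline drives a self-resetting DoN counter that alternates between two creak sounds at the door's location.
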(event OnOpenRequest97(OpenDoor)
  (bind _returnvalue (Transformation|GetActorLocation))
  (bind _open_angle (Timeline|Door%20Swing Play)
    (:Update
      (Transformation|SetActorRotation (Math|Rotator|Lerp(Rotator) (Variables|Default|GetInitialRotation) (Variables|Default|GetNewVar_0) _open_angle)))
    (:Sounds
      (bind _counter (Utilities|FlowControl|DoN 2 :!label _label)
        (:Exit
          (switch int _counter
            (:1
              (Audio|PlaySoundatLocation "/Game/Sounds/creaky-door-open4.creaky-door-open4" _returnvalue "0, 0, 0" 1.0 1.0 0.0 0 0 0))
            (:2
              (Audio|PlaySoundatLocation "/Game/Sounds/creaky-door-open5.creaky-door-open5" _returnvalue "0, 0, 0" 1.0 1.0 0.0 0 0 0)
              (goto _label Reset))))))))

(event OnCloseRequest97(OpenDoor)
  (bind _returnvalue (Transformation|GetActorLocation))
  (bind _open_angle (Timeline|Door%20Swing Reverse)
    (:Update
      (Transformation|SetActorRotation (Math|Rotator|Lerp(Rotator) (Variables|Default|GetInitialRotation) (Variables|Default|GetNewVar_0) _open_angle)))
    (:Sounds
      (bind _counter (Utilities|FlowControl|DoN 2 :!label _label)
        (:Exit
          (switch int _counter
            (:1
              (Audio|PlaySoundatLocation "/Game/Sounds/creaky-door-open4.creaky-door-open4" _returnvalue "0, 0, 0" 1.0 1.0 0.0 0 0 0))
            (:2
              (Audio|PlaySoundatLocation "/Game/Sounds/creaky-door-open5.creaky-door-open5" _returnvalue "0, 0, 0" 1.0 1.0 0.0 0 0 0)
              (goto _label Reset))))))))

(event EventBeginPlay
  (Variables|Default|SetInitialRotation (Transformation|GetActorRotation)))

(fn ConstructionScript)